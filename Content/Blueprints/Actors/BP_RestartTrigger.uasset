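; BP_RestartTrigger is a trigger actor that restarts the current level when the player's pawn overlaps it.
; On overlap by player 0's pawn, it fades the camera out and holds the fade.
; After a delay slightly longer than the fade, it reopens the current level by name, fully reloading it.
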(event `self.ReceiveActorBeginOverlap`
  (params (OtherActor :type "Actor Object Reference"))
  (if (== OtherActor (`GameplayStatics.GetPlayerPawn` 0))
    (`PlayerCameraManager.StartCameraFade` :`self` (`GameplayStatics.GetPlayerCameraManager` 0) :`ToAlpha` 1.0 :`Duration` 0.5 :`bHoldWhenFinished` true)
    (`KismetSystemLibrary.Delay` (+ 0.5 0.25))
    (bind _returnvalue (`GameplayStatics.GetCurrentLevelName` true))
    (`GameplayStatics.OpenLevel` (`KismetStringLibrary.Conv_StringToName` _returnvalue))))

(fn `UserConstructionScript`)