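; BP_PlayerPawn is a player pawn that moves by rolling its Ball component with physics.
; Forward/backward and left/right axis inputs, scaled by MoveSpeed, apply torque on the Y and X axes as an acceleration change, so mass does not affect the response.
; On BeginPlay, the player camera manager briefly fades the view in.
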(event `self.ReceiveBeginPlay`
  (`PlayerCameraManager.StartCameraFade` :`self` (`GameplayStatics.GetPlayerCameraManager` 0) :`FromAlpha` 1.0 :`Duration` 0.5))

(event `InputAxis|Move Forward/Backward`
  (params (AxisValue :type "Float (single-precision)"))
  (`PrimitiveComponent.AddTorqueInRadians` (`self.Ball`) (`KismetMathLibrary.MakeVector` 0.0 (* AxisValue (`self.MoveSpeed`))) "None" true))

(event `InputAxis|Move Left/Right`
  (params (AxisValue :type "Float (single-precision)"))
  (`PrimitiveComponent.AddTorqueInRadians` (`self.Ball`) (`KismetMathLibrary.MakeVector` (* AxisValue (`self.MoveSpeed`))) "None" true))

(fn `UserConstructionScript`)